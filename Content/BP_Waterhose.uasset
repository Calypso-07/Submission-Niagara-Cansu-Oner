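; Water hose actor that follows the player's camera and sprays Niagara water while left mouse is held, extinguishing fires.
; A looping timer updates its position and spray direction.
; Exported particle positions are checked at intervals against actors tagged "Extinguishable", draining per-fire strength stored in a map.
; That strength scales each fire's Niagara spawn rate, and throttled steam effects spawn at hits while fire remains.
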(event `self.ReceiveBeginPlay`
  (`parent.ReceiveBeginPlay`)
  (bind _outactors (`GameplayStatics.GetAllActorsWithTag` "Extinguishable"))
  (`KismetSystemLibrary.PrintString` (`KismetStringLibrary.Conv_IntToString` (`KismetArrayLibrary.Array_Length` _outactors)))
  (bind _output_get (set `self.FireActors` _outactors))
  (for _array_element _output_get
    (`BlueprintMapLibrary.Map_Add` (`self.Firehealth`) _array_element 1.0))
  (`self.EnableInput` (`GameplayStatics.GetPlayerController` 0))
  (`KismetSystemLibrary.K2_SetTimerDelegate` (delegate `UpdateWaterPose`) 0.02 true))

(event `self.ReceiveParticleData`
  (params (Data :type "Array of BasicParticleData Structure (by ref)") (NiagaraSystem :type "NiagaraSystem Object Reference") (SimulationPositionOffset :type "Vector Structure (by ref)"))
  (bind _output_get (set `self.FireCheckDelta` (- (`KismetSystemLibrary.GetGameTimeInSeconds`) (`self.LastFireCheckTiem`))))
  (if (>= _output_get (`self.FireCheckInterval`))
    (set `self.LastFireCheckTiem` (`KismetSystemLibrary.GetGameTimeInSeconds`))
    (set `self.cached` Data)
    (for _array_element (`self.FireActors`)
      (bind _output_get_2 (set `self.FireActor` _array_element))
      (bind _output_get_3 (set `self.FireStrength` (`BlueprintMapLibrary.Map_Find` (`self.Firehealth`) _output_get_2)))
      (if (> _output_get_3 0.0)
        (`/Engine/EditorBlueprintResources/StandardMacros.IsValid` (`self.FireActor`)
          (:`Is Valid`
            (for _array_element_2 (`self.cached`)
              (bind _returnvalue (+ (`.Position` (break `BasicParticleData` _array_element_2)) SimulationPositionOffset))
              (if (<= (`KismetMathLibrary.Vector_Distance` _returnvalue (+ (`self.K2_GetActorLocation` (`self.FireActor`)) (`self.FireCenterOffset`))) (`self.FireRadius`))
                (bind _output_get_4 (set `self.FireStrength` (`KismetMathLibrary.FClamp` (- (`self.FireStrength`) (/ (`KismetMathLibrary.FMin` (`self.FireCheckDelta`) 0.1) (`self.ExtinguishSeconds`))))))
                (`BlueprintMapLibrary.Map_Add` (`self.Firehealth`) (`self.FireActor`) _output_get_4)
                (`NiagaraComponent.SetVariableFloat` (`self.GetComponentByClass` (`self.FireActor`) "/Script/Niagara.NiagaraComponent") "User.FireSpawnRate" (* (`self.InitialFireSpawnRate`) (`self.FireStrength`)))
                (if (and (> (`self.FireStrength`) 0.0) (>= (- (`KismetSystemLibrary.GetGameTimeInSeconds`) (`self.LastSteamTime`)) (`self.SteamInterval`)))
                  (set `self.LastSteamTime` (`KismetSystemLibrary.GetGameTimeInSeconds`))
                  (`NiagaraFunctionLibrary.SpawnSystemAtLocation` "/Game/NS_Steam.NS_Steam" _returnvalue)
                  (break)
                  (else
                    (break)))))))))))

(event `Key|LeftMouseButton`
  (params (Key :type "Key Structure"))
  (:`Pressed`
    (`NiagaraComponent.SetVariableFloat` (`self.WaterNiagara`) "User.WaterSpawnRate" 2000.0))
  (:`Released`
    (`NiagaraComponent.SetVariableFloat` (`self.WaterNiagara`) "User.WaterSpawnRate" 0.0)))

(event `UpdateWaterPose`
  (bind _returnvalue (`GameplayStatics.GetPlayerCharacter` 0))
  (bind _returnvalue_2 (`PlayerCameraManager.GetCameraRotation` (`GameplayStatics.GetPlayerCameraManager` 0)))
  (bind _returnvalue_3 (`KismetMathLibrary.GetForwardVector` _returnvalue_2))
  (`/Engine/EditorBlueprintResources/StandardMacros.IsValid` _returnvalue
    (:`Is Valid`
      (`self.K2_SetActorLocation` (+ (`self.K2_GetActorLocation` _returnvalue) (+ (+ (* _returnvalue_3 80.0) (* (`KismetMathLibrary.GetRightVector` _returnvalue_2) 25.0)) (`KismetMathLibrary.MakeVector` 0.0 0.0 40.0))))
      (`NiagaraComponent.SetVariableVec3` (`self.WaterNiagara`) "User.WaterDirection" (+ _returnvalue_3 (0.0 0.0 1.0))))))

(fn `UserConstructionScript`)